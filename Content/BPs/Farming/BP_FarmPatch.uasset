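; BP_FarmPatch is an unfinished farmland tile that plants a crop when a Cube actor enters its box.
; Box overlap sets IsFarmland, then spawns BP_Cauliflower at the Cube's location.
; Left-click state is recorded but does not gate planting, and the occupancy check only prints without blocking spawns.
; End overlap sets IsFarmland true despite its comment saying it clears the flag.
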(event `Key|LeftMouseButton`
  (params (Key :type "Key Structure"))
  ; This hopefully makes left click plant a crop only inside farmland - Tom.
  (:`Pressed`
    (set `self.LMBPressed` true)
    (`KismetSystemLibrary.PrintString` "LMB Pressed" true true (struct :`R` 1.0 :`G` 0.968377 :`B` 0.978093 :`A` 1.0)))
  (:`Released`
    (set `self.LMBPressed` false)
    (`KismetSystemLibrary.PrintString` "LMB Released" true true (struct :`R` 1.0 :`G` 0.968377 :`B` 0.978093 :`A` 1.0))))

(event `self.Box.OnComponentBeginOverlap`
  (params (OverlappedComponent :type "PrimitiveComponent Object Reference") (OtherActor :type "Actor Object Reference") (OtherComp :type "PrimitiveComponent Object Reference") (OtherBodyIndex :type Integer) (bFromSweep :type Boolean) (SweepResult :type "HitResult Structure (by ref)"))
  ; Crop spawn - unfinished (Trying to add click detection that activates the growth) - Tom and Ben.
  (bind _ascube (cast `/Game/BPs/WorldGridBP/Cube` OtherActor))
  (set `self.IsFarmland` true)
  (`KismetSystemLibrary.PrintString` "InFarmland" true true (struct :`R` 1.0 :`G` 0.848956 :`A` 1.0))
  (`self.IsOccupiedCheck`) ; Function to check your tile is unused by other crops.
  (`KismetSystemLibrary.PrintString` "Ready" true true (struct :`G` 1.0 :`B` 0.125573 :`A` 1.0))
  (if (`self.IsFarmland`)
    (`KismetSystemLibrary.PrintString` "Hello")
    (`|SpawnActorFromClass` "/Game/BPs/Farming/BP_Cauliflower.BP_Cauliflower_C" (`KismetMathLibrary.MakeTransform` (`self.K2_GetActorLocation` _ascube) (struct) (1.5 1.5 1.0)) "AlwaysSpawn" "MultiplyWithRoot" null null)
    (`KismetSystemLibrary.PrintString` "CROP PLANTED" true true (struct :`R` 0.993489 :`G` 0.039163 :`B` 1.0 :`A` 1.0))))

(event `self.Box.OnComponentEndOverlap`
  (params (OverlappedComponent :type "PrimitiveComponent Object Reference") (OtherActor :type "Actor Object Reference") (OtherComp :type "PrimitiveComponent Object Reference") (OtherBodyIndex :type Integer))
  ; Crop spawn - unfinished (Trying to add click detection that activates the growth) - Tom and Ben.
  ;; Removes "Farmland" boolean when you leave it to avoid bugs. - Tom.
  (set `self.IsFarmland` true)
  (`KismetSystemLibrary.PrintString` "NotInFarmland" true true (struct :`R` 1.0 :`G` 0.848956 :`A` 1.0)))

(fn `IsOccupiedCheck`
  (if (not (`self.IsOccupied`))
    (`KismetSystemLibrary.PrintString` "IsNotOccupied")
    (return)))

(fn `UserConstructionScript`)