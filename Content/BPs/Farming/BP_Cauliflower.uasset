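; BP_Cauliflower is a farming crop that grows through five visual stages after it begins play.
; A one-shot chain of timed delays toggles the visibility of consecutive stage components to swap each stage for the next.
; At the final stage it sets IsGrown to true and prints a debug message.
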(event `self.ReceiveBeginPlay`
  ; Growth Sequence - Ben
  (set `self.IsGrown` false)
  (`/Engine/EditorBlueprintResources/StandardMacros.DoOnce` false
    (:`Completed`
      (`KismetSystemLibrary.Delay` 3.0)
      (`SceneComponent.ToggleVisibility` (`self.Stage1`) false)
      (`SceneComponent.ToggleVisibility` (`self.Stage2`) false)
      (`KismetSystemLibrary.Delay` 3.0)
      (`SceneComponent.ToggleVisibility` (`self.Stage2`) false)
      (`SceneComponent.ToggleVisibility` (`self.Stage3`) false)
      (`KismetSystemLibrary.Delay` 3.0)
      (`SceneComponent.ToggleVisibility` (`self.Stage3`) false)
      (`SceneComponent.ToggleVisibility` (`self.Stage4`) false)
      (`KismetSystemLibrary.Delay` 3.0)
      (`SceneComponent.ToggleVisibility` (`self.Stage4`) false)
      (`SceneComponent.ToggleVisibility` (`self.Stage5`) false)
      (set `self.IsGrown` true)
      (`KismetSystemLibrary.PrintString` "CropGrown" true true (struct :`R` 0.401647 :`G` 1.0 :`B` 0.001142 :`A` 1.0)))))

(fn `UserConstructionScript`)